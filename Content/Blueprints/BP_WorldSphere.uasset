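; BP_WorldSphere is a rotatable globe actor that displays a map of a BurinWorld on its sphere mesh.
; BeginPlay creates the world, a 4096 render target bound to a dynamic material, and a MapLowZoom helper.
; RenderVcMapBP draws MapLowZoom's triangles for a given map mode onto that target's canvas.
; RotateWorldSphere accumulates yaw and clamped pitch, then rebuilds rotation from zero, with Up feeding yaw and Right feeding pitch.
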(event EventBeginPlay
  (Utilities|FlowControl|Sequence
    (:then_0
      (bind _returnvalue (Game|ConstructObjectfromClass "/Script/VectorMapTest.BurinWorld"))
      (bind _output_get (Variables|Default|SetBurinWorld _returnvalue))
      (Class|BurinWorld|Initialize _output_get))
    (:then_1
      (bind _returnvalue_2 (Rendering|CreateRenderTarget2D 4096 4096 "RTF_RGBA16f"))
      (bind _output_get_2 (Variables|Default|SetRenderTarget _returnvalue_2))
      (Rendering|ClearRenderTarget2D _output_get_2 "(R=0.008743,G=0.298097,B=1.000000,A=1.000000)"))
    (:then_2
      (bind _returnvalue_3 (Rendering|Material|CreateDynamicMaterialInstance "/Game/Materials/WorldCanvasMat.WorldCanvasMat" "None" "None" :!class /Script/Engine.KismetMaterialLibrary))
      (Rendering|Material|SetTextureParameterValue _returnvalue_3 "WorldCanvasTexture" (Variables|Default|GetRenderTarget))
      (Rendering|Material|SetMaterial (Variables|Components|GetSphere) 0 _returnvalue_3))
    (:then_3
      (bind _returnvalue_4 (Game|ConstructObjectfromClass "/Script/VectorMapTest.MapLowZoom"))
      (Variables|Default|SetMapLowZoom _returnvalue_4)
      (CallFunction|RenderVcMapBP))))

(event Collision|EventActorBeginOverlap
  (params (OtherActor :type Actor%20Object%20Reference)))

(event EventTick
  (params (DeltaSeconds :type Float%20%28single-precision%29)))

(fn ConstructionScript)

(fn RenderVcMapBP
  (params (MapMode :type Integer))
  (bind _rendertarget (Variables|Default|GetRenderTarget))
  (Rendering|ClearRenderTarget2D _rendertarget)
  (bind (_canvas _size _context) (Rendering|BeginDrawCanvastoRenderTarget _rendertarget))
  (Development|PrintString "Hello")
  (bind _returnvalue (Class|MapLowZoom|GetTriangles (Variables|Default|GetMapLowZoom) (Variables|Default|GetBurinWorld) MapMode))
  (Class|Canvas|DrawTriangle _canvas 0 _returnvalue)
  (Rendering|EndDrawCanvastoRenderTarget _context))

(fn RotateWorldSphere
  (params (Right :type Float%20%28double-precision%29) (Up :type Float%20%28double-precision%29))
  (Variables|Default|SetRightRot (+ Up (Variables|Default|GetRightRot)))
  (Variables|Default|SetUpRot (Math|Float|Min(Float) (Math|Float|Max(Float) (+ (Variables|Default|GetUpRot) Right) -8e+01) 8e+01))
  (Transformation|SetActorRotation "0, 0, 0")
  (Transformation|AddActorLocalRotation (Math|Rotator|MakeRotator 0.0 (Variables|Default|GetUpRot) 0.0) false false)
  (Transformation|AddActorLocalRotation (Math|Rotator|MakeRotator 0.0 0.0 (Variables|Default|GetRightRot)) false false))